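; BP_BaseUnit is a unit actor that repeatedly moves itself toward the nearest BP_Gatherable.
; A looping timer refreshes the list of gatherables and sets the nearest one's location as the target.
; A timeline lerps from start to target without sweep or pathfinding, then resets the start and replays.
; While the cached list is empty, the unit holds position and zeroes the target.
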(event `MoveToGatherable`
  (bind (_direction _floattrack) (`Timeline|MoveToResource` :`NewTime` 2.0 :!via `PlayFromStart`)
    (:`Update`
      (if (`KismetArrayLibrary.Array_IsNotEmpty` (stale `FindGatherables` _outactors))
        (`self.K2_SetActorLocation` (`KismetMathLibrary.VLerp` (`self.StartLocation`) (`self.TargetLocation`) _floattrack))
        (else
          (set `self.TargetLocation` (0.0 0.0 0.0)))))
    (:`Finished`
      (set `self.StartLocation` (`self.K2_GetActorLocation`))
      (`self.MoveToGatherable`))))

(event `self.ReceiveBeginPlay`
  (bind _returnvalue_location (`KismetMathLibrary.BreakTransform` (`self.GetTransform`)))
  (set `self.StartLocation` _returnvalue_location)
  (`|ExecutionSequence`
    (:`then_0`
      (`self.MoveToGatherable`))
    (:`then_1`
      (`KismetSystemLibrary.K2_SetTimer` null "FindGatherables" 2.0 true false 2.0))))

(event `FindGatherables`
  (bind _outactors (`GameplayStatics.GetAllActorsOfClass` "/Game/BP_Gatherable.BP_Gatherable_C"))
  (set `self.TargetLocation` (`self.K2_GetActorLocation` (`.ReturnValue` (`GameplayStatics.FindNearestActor` (`self.K2_GetActorLocation`) _outactors)))))

(fn `UserConstructionScript`)