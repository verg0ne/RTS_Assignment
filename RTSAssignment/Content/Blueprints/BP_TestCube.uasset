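; BP_TestCube is a test placement preview cube that follows the mouse cursor and shows whether it is within range of a home base.
; BeginPlay stores the actor tagged HomeBase, keeping the last if several exist.
; Each tick it moves to the X and Y of a visibility trace under the cursor.
; It switches to a not-placeable material when its distance from the base exceeds MaxDistance.
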(event `self.ReceiveBeginPlay`
  (bind _outactors (`GameplayStatics.GetAllActorsWithTag` "HomeBase"))
  (for _array_element _outactors
    (set `self.Base` _array_element)))

(event `self.ReceiveTick`
  (params (DeltaSeconds :type "Float (single-precision)"))
  (bind _hitresult (`PlayerController.GetHitResultUnderCursorByChannel` (`GameplayStatics.GetPlayerController` 0) "TraceTypeQuery1" true))
  (`self.K2_SetActorLocation` (`KismetMathLibrary.MakeVector` (.x (`.Location` (`GameplayStatics.BreakHitResult` _hitresult))) (.y (`.Location` (`GameplayStatics.BreakHitResult` _hitresult)))))
  (if (> (`KismetMathLibrary.Vector_Distance` (`self.K2_GetActorLocation`) (`self.K2_GetActorLocation` (`self.Base`))) (`self.MaxDistance`))
    (`PrimitiveComponent.SetMaterial` (`self.Cube`) 0 "/Game/Materials/M_NotPlaceable.M_NotPlaceable")
    (else
      (`PrimitiveComponent.SetMaterial` (`self.Cube`) 0 "/Engine/MapTemplates/Materials/BasicAsset03.BasicAsset03"))))

(fn `UserConstructionScript`)