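; BP_Meteor is a projectile actor that flies at the nearest unit and explodes on impact.
; On BeginPlay it records the location of the closest BP_BaseUnit once, so it does not track movement.
; A timeline lerps it from its current location toward that point.
; Overlapping an actor tagged Multiplier or Gatherer applies fixed damage, spawns a scaled-up Niagara explosion and destroys the meteor.
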(event `self.ReceiveBeginPlay`
  (bind _outactors (`GameplayStatics.GetAllActorsOfClass` "/Game/Blueprints/BP_BaseUnit.BP_BaseUnit_C"))
  (set `self.TargetPosition` (`self.K2_GetActorLocation` (`.ReturnValue` (`GameplayStatics.FindNearestActor` (`self.K2_GetActorLocation`) _outactors))))
  (bind (_direction _floattrack) (`Timeline|MoveToTarget` :!via `PlayFromStart`)
    (:`Update`
      (`self.K2_SetActorLocation` (`KismetMathLibrary.VLerp` (`self.K2_GetActorLocation`) (`self.TargetPosition`) _floattrack)))))

(event `self.ReceiveActorBeginOverlap`
  (params (OtherActor :type "Actor Object Reference"))
  (bind (_returnvalue_location _returnvalue_rotation) (`KismetMathLibrary.BreakTransform` (`self.GetTransform`)))
  (if (or (`self.ActorHasTag` OtherActor "Multiplier") (`self.ActorHasTag` OtherActor "Gatherer"))
    (`GameplayStatics.ApplyDamage` OtherActor 33.0)
    (`NiagaraFunctionLibrary.SpawnSystemAtLocation` "/Game/Niagara/NS_Explosion.NS_Explosion" _returnvalue_location _returnvalue_rotation (10.0 10.0 10.0))
    (`self.K2_DestroyActor`)))

(fn `UserConstructionScript`)