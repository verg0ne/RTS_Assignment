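; Base gatherer unit that shuttles between BP_Gatherable actors and the world origin, firing OnGoldDeposited when it overlaps a HomeBase while carrying.
; FindGatherables claims an untargeted gatherable passing a summed X/Y offset threshold, or falls back to the origin.
; MoveToGatherable lerps location with a timeline, toggles HasGathered on arrival and searches again.
; Damage lowers Health and swaps the box material at half-health and dying thresholds.
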(event `self.ReceiveActorBeginOverlap`
  (params (OtherActor :type "Actor Object Reference"))
  ;[0.15 0.1239 0.01947 0.5] Deposit Gold
  (if (and (`self.ActorHasTag` OtherActor "HomeBase") (`self.bHasGathered`))
    (`KismetSystemLibrary.PrintString` "Depositing")
    (`self.OnGoldDeposited`)))

(event `self.ReceiveAnyDamage`
  (params (Damage :type "Float (single-precision)") (DamageType :type "DamageType Object Reference") (InstigatedBy :type "Controller Object Reference") (DamageCauser :type "Actor Object Reference"))
  ;[0.15 0.001032 0.02754 0.5] Damage
  (bind _output_get (set `self.Health` (- (`self.Health`) Damage)))
  (if (> _output_get 67.0)
    _
    (elif (> (`self.Health`) 34.0)
      (`PrimitiveComponent.SetMaterial` (`self.Box`) 0 "/Game/Materials/M_HalfHealth.M_HalfHealth")
      (else
        (`PrimitiveComponent.SetMaterial` (`self.Box`) 0 "/Game/Materials/M_Dying.M_Dying")))))

(event `MoveToGatherable`
  (bind _returnvalue_location (`KismetMathLibrary.BreakTransform` (`self.GetTransform`)))
  (bind _targetlocation (`self.TargetLocation`))
  (bind _targetlocation_2 (`self.TargetLocation`))
  (bind (_returnvalue_x _returnvalue_y) (`KismetMathLibrary.BreakVector` (/ (`self.StartLocation`) _targetlocation_2)))
  (set `self.StartLocation` _returnvalue_location)
  (if (`KismetMathLibrary.Vector_IsZero` _targetlocation_2)
    (set `self.TargetLocation` (0.0 0.0 0.0))
    (bind (_direction _floattrack) (`Timeline|MoveToResource` :`NewTime` (+ _returnvalue_x _returnvalue_y) :!via `PlayFromStart` :!label _label)
      (:`Update`
        (set `self.bIsMoving` true)
        (if (`AIBlueprintHelperLibrary.IsValidAILocation` _targetlocation)
          (`self.K2_SetActorLocation` (`KismetMathLibrary.VLerp` (`self.StartLocation`) _targetlocation _floattrack))))
      (:`Finished`
        (set `self.StartLocation` (`self.K2_GetActorLocation`))
        (set `self.bIsMoving` false)
        (if (`self.bHasGathered`)
          (set `self.bHasGathered` false)
          (else
            (set `self.bHasGathered` true)))
        (`self.FindGatherables`)))
    (else
      (goto _label :!via `PlayFromStart`))))

(event `self.ReceiveBeginPlay`
  (`self.FindGatherables`))

(event `FindGatherables`
  (bind _finaltarget (`self.FinalTarget`))
  (if (not (`self.bIsMoving`))
    (bind _outactors (`GameplayStatics.GetAllActorsOfClass` "/Game/Blueprints/BP_Gatherable.BP_Gatherable_C"))
    (for _array_element _outactors
      (bind _returnvalue (`self.K2_GetActorLocation` _array_element))
      (bind (_returnvalue_x _returnvalue_y) (`KismetMathLibrary.BreakVector` (- (`self.K2_GetActorLocation`) _returnvalue)))
      (if (and (<= (+ _returnvalue_x _returnvalue_y) (`self.closestDistance`)) (not (`/Game/Blueprints/BP_Gatherable.bIsTargeted` _array_element)))
        (set `self.TargetLocation` _returnvalue)
        (set `self.FinalTarget` _array_element)))
    (if (`self.bHasGathered`)
      (set `self.TargetLocation` (0.0 0.0 0.0) :!label _label_2)
      (else
        (`/Engine/EditorBlueprintResources/StandardMacros.IsValid` _finaltarget
          (:`Is Valid`
            (if (`/Game/Blueprints/BP_Gatherable.bIsTargeted` _finaltarget)
              (goto _label_2)
              (else
                (set `/Game/Blueprints/BP_Gatherable.bIsTargeted` true (`self.FinalTarget`)))))
          (:`Is Not Valid`
            (`KismetSystemLibrary.PrintString` "Invalid Target")
            (goto _label_2)))))
    (`self.MoveToGatherable`)))

(fn `MoveTo`)

(fn `UserConstructionScript`)